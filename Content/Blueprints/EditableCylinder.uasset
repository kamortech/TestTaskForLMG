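; Editable cylinder building piece that the player can pick up, reposition, rotate and scale while construct mode is active on the Green_cube actor.
; Interact toggles holding by attaching it to the player camera manager and teleporting it near the character, or detaching it in place.
; While held, input actions nudge its transform in fixed world-axis steps.
; Each action repeats through a Gate and short Delay loop until its key is released.
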(event `/Game/Blueprints/InteractionInterface.Interact`
  (bind _returnvalue (`GameplayStatics.GetPlayerCharacter` 0))
  ;[1 1 1] Interaction
  (bind _outactors (`GameplayStatics.GetAllActorsOfClass` "/Game/Blueprints/green_cube.green_cube_C"))
  (if (`/Game/Blueprints/green_cube.isConstructModeActive` (`|GetArrayItem` _outactors))
    (if (`self.isHeld`)
      (`KismetSystemLibrary.PrintString` "Releasing object...")
      (`self.K2_DetachFromActor` "KeepWorld" "KeepWorld" "KeepWorld")
      (set `self.isHeld` false)
      (else
        (set `self.isHeld` true)
        (`KismetSystemLibrary.PrintString` "Basic Cylinder Piecked!" true true (struct :`G` 0.552083 :`B` 0.011629 :`A` 1.0))
        (`self.K2_AttachToActor` (`GameplayStatics.GetPlayerCameraManager` 0) "None" "KeepWorld" "KeepWorld" "KeepWorld")
        (`self.K2_TeleportTo` (+ (`self.K2_GetActorLocation` _returnvalue) (0.0 -12.0 0.0)) (`self.K2_GetActorRotation` _returnvalue))))
    (else
      (`KismetSystemLibrary.PrintString` "To Construct You must use Drawing Board!" true true (struct :`R` 0.744792 :`B` 0.005153 :`A` 1.0)))))

(event `InputAction|RotateLeft` :consume false
  (params (Key :type "Key Structure"))
  ;[1 1 1] Rotation to Left
  (:`Pressed`
    (if (`self.isHeld`)
      (`|ExecutionSequence`
        (:`then_0`
          (goto _label :!via `Open`))
        (:`then_1`
          (`/Engine/EditorBlueprintResources/StandardMacros.Gate` true :!label _label
            (:`Exit`
              (`self.K2_SetActorRotation` (`KismetMathLibrary.Conv_VectorToRotator` (+ (`KismetMathLibrary.Conv_RotatorToVector` (`self.K2_GetActorRotation` self)) (0.0 0.05 0.0))))
              (`KismetSystemLibrary.Delay` 0.05)
              (goto _label)))))))
  (:`Released`
    (goto _label :!via `Close`)))

(event `InputAction|TransformForward` :consume false
  (params (Key :type "Key Structure"))
  ;[1 1 1] Transforming Forward
  (:`Pressed`
    (if (`self.isHeld`)
      (`|ExecutionSequence`
        (:`then_0`
          (goto _label_2 :!via `Open`))
        (:`then_1`
          (`/Engine/EditorBlueprintResources/StandardMacros.Gate` true :!label _label_2
            (:`Exit`
              (`self.K2_SetActorLocation` (+ (`self.K2_GetActorLocation` self) (0.0 1.0 0.0)))
              (`KismetSystemLibrary.Delay` 0.05)
              (goto _label_2)))))))
  (:`Released`
    (goto _label_2 :!via `Close`)))

(event `InputAction|ScaleUP` :consume false
  (params (Key :type "Key Structure"))
  ;[1 1 1] Scaling Up
  (:`Pressed`
    (if (`self.isHeld`)
      (`|ExecutionSequence`
        (:`then_0`
          (goto _label_3 :!via `Open`))
        (:`then_1`
          (`/Engine/EditorBlueprintResources/StandardMacros.Gate` true :!label _label_3
            (:`Exit`
              (`self.SetActorScale3D` (+ (`self.GetActorScale3D` self) (0.05 0.05 0.05)))
              (`KismetSystemLibrary.Delay` 0.05)
              (goto _label_3)))))))
  (:`Released`
    (goto _label_3 :!via `Close`)))

(event `InputAction|RotateRight` :consume false
  (params (Key :type "Key Structure"))
  ;[1 1 1] Rotation to Right
  (:`Pressed`
    (if (`self.isHeld`)
      (`|ExecutionSequence`
        (:`then_0`
          (goto _label_4 :!via `Open`))
        (:`then_1`
          (`/Engine/EditorBlueprintResources/StandardMacros.Gate` true :!label _label_4
            (:`Exit`
              (`self.K2_SetActorRotation` (`KismetMathLibrary.Conv_VectorToRotator` (+ (`KismetMathLibrary.Conv_RotatorToVector` (`self.K2_GetActorRotation` self)) (0.0 -0.05 0.0))))
              (`KismetSystemLibrary.Delay` 0.05)
              (goto _label_4)))))))
  (:`Released`
    (goto _label_4 :!via `Close`)))

(event `InputAction|TransformBackward` :consume false
  (params (Key :type "Key Structure"))
  ;[1 1 1] Transforming Backward
  (:`Pressed`
    (if (`self.isHeld`)
      (`|ExecutionSequence`
        (:`then_0`
          (goto _label_5 :!via `Open`))
        (:`then_1`
          (`/Engine/EditorBlueprintResources/StandardMacros.Gate` true :!label _label_5
            (:`Exit`
              (`self.K2_SetActorLocation` (+ (`self.K2_GetActorLocation` self) (0.0 -1.0 0.0)))
              (`KismetSystemLibrary.Delay` 0.05)
              (goto _label_5)))))))
  (:`Released`
    (goto _label_5 :!via `Close`)))

(event `InputAction|ScaleDown` :consume false
  (params (Key :type "Key Structure"))
  ;[1 1 1] Scaling Down
  (:`Pressed`
    (if (`self.isHeld`)
      (`|ExecutionSequence`
        (:`then_0`
          (goto _label_6 :!via `Open`))
        (:`then_1`
          (`/Engine/EditorBlueprintResources/StandardMacros.Gate` true :!label _label_6
            (:`Exit`
              (`self.SetActorScale3D` (+ (`self.GetActorScale3D` self) (-0.05 -0.05 -0.05)))
              (`KismetSystemLibrary.Delay` 0.05)
              (goto _label_6)))))))
  (:`Released`
    (goto _label_6 :!via `Close`)))

(event `InputAction|TransformLeft` :consume false
  (params (Key :type "Key Structure"))
  ;[1 1 1] Transforming to Left
  (:`Pressed`
    (if (`self.isHeld`)
      (`|ExecutionSequence`
        (:`then_0`
          (goto _label_7 :!via `Open`))
        (:`then_1`
          (`/Engine/EditorBlueprintResources/StandardMacros.Gate` true :!label _label_7
            (:`Exit`
              (`self.K2_SetActorLocation` (+ (`self.K2_GetActorLocation` self) (1.0 0.0 0.0)))
              (`KismetSystemLibrary.Delay` 0.05)
              (goto _label_7)))))))
  (:`Released`
    (goto _label_7 :!via `Close`)))

(event `InputAction|TransformRight` :consume false
  (params (Key :type "Key Structure"))
  ;[1 1 1] Transforming to Right
  (:`Pressed`
    (if (`self.isHeld`)
      (`|ExecutionSequence`
        (:`then_0`
          (goto _label_8 :!via `Open`))
        (:`then_1`
          (`/Engine/EditorBlueprintResources/StandardMacros.Gate` true :!label _label_8
            (:`Exit`
              (`self.K2_SetActorLocation` (+ (`self.K2_GetActorLocation` self) (-1.0 0.0 0.0)))
              (`KismetSystemLibrary.Delay` 0.05)
              (goto _label_8)))))))
  (:`Released`
    (goto _label_8 :!via `Close`)))

(fn `UserConstructionScript`)