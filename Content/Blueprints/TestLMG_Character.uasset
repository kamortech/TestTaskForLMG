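; TestLMG_Character is a player Character Blueprint that handles basic look, movement and jump input.
; Look axes drive controller yaw and pitch, and the Jump action calls Jump on press with no release handler.
; Forward movement follows the control rotation with pitch zeroed, while strafing uses the right vector of the full control rotation.
; The Construction Script is empty.
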(event `InputAxis|LookRight`
  (params (AxisValue :type "Float (single-precision)"))
  ;[1 1 1] Mouse Movement Control
  (`self.AddControllerYawInput` AxisValue))

(event `InputAxis|MoveRight`
  (params (AxisValue :type "Float (single-precision)"))
  ;[1 1 1] Keyboard Movement Control
  (`self.AddMovementInput` (`KismetMathLibrary.GetRightVector` (`self.GetControlRotation`)) AxisValue))

(event `InputAxis|MoveForward`
  (params (AxisValue :type "Float (single-precision)"))
  ;[1 1 1] Keyboard Movement Control
  (`self.AddMovementInput` (`KismetMathLibrary.GetForwardVector` (`KismetMathLibrary.MakeRotator` (.roll (`self.GetControlRotation`)) 0.0 (.yaw (`self.GetControlRotation`)))) AxisValue))

(event `InputAxis|LookUP`
  (params (AxisValue :type "Float (single-precision)"))
  ;[1 1 1] Mouse Movement Control
  (`self.AddControllerPitchInput` AxisValue))

(event `InputAction|Jump`
  (params (Key :type "Key Structure"))
  ;[1 1 1] Keyboard Jump
  (:`Pressed`
    (`self.Jump`)))

(fn `UserConstructionScript`)