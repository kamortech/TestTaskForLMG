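; EditableCube is a construction cube actor that the player can pick up and drop while construct mode is active.
; Interact checks the first Green_cube actor's mode flag, then toggles between attaching the cube to the camera manager with a teleport near the player and detaching it in place.
; Holding TransformForward runs a Gate and Delay loop that nudges the cube along world Y, independent of grab state or construct mode.
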(event `/Game/Blueprints/InteractionInterface.Interact`
  (bind _returnvalue (`GameplayStatics.GetPlayerCharacter` 0))
  (bind _outactors (`GameplayStatics.GetAllActorsOfClass` "/Game/Blueprints/green_cube.green_cube_C"))
  (if (`/Game/Blueprints/green_cube.isConstructModeActive` (`|GetArrayItem` _outactors))
    (if (`self.isGrabbed`)
      (`KismetSystemLibrary.PrintString` "Releasing object...")
      (`self.K2_DetachFromActor` "KeepWorld" "KeepWorld" "KeepWorld")
      (set `self.isGrabbed` false)
      (else
        (set `self.isGrabbed` true)
        (`KismetSystemLibrary.PrintString` "Basic Cube Piecked!" true true (struct :`G` 0.552083 :`B` 0.011629 :`A` 1.0))
        (`self.K2_AttachToActor` (`GameplayStatics.GetPlayerCameraManager` 0) "None" "KeepWorld" "KeepWorld" "KeepWorld")
        (`self.K2_TeleportTo` (+ (`self.K2_GetActorLocation` _returnvalue) (0.0 -12.0 0.0)) (`self.K2_GetActorRotation` _returnvalue))))
    (else
      (`KismetSystemLibrary.PrintString` "To Construct You must use Drawing Board!" true true (struct :`R` 0.744792 :`B` 0.005153 :`A` 1.0)))))

(event `InputAction|TransformForward`
  (params (Key :type "Key Structure"))
  (:`Pressed`
    (`|ExecutionSequence`
      (:`then_0`
        (goto _label :!via `Open`))
      (:`then_1`
        (`/Engine/EditorBlueprintResources/StandardMacros.Gate` true :!label _label
          (:`Exit`
            (`KismetSystemLibrary.PrintString` "Hello")
            (`self.K2_SetActorLocation` (+ (`self.K2_GetActorLocation` self) (0.0 1.0 0.0)))
            (`KismetSystemLibrary.Delay` 0.05)
            (goto _label))))))
  (:`Released`
    (goto _label :!via `Close`)))

(fn `UserConstructionScript`)